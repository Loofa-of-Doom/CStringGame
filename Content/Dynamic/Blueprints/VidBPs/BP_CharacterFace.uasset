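; BP_CharacterFace is a player-controlled face character that slides horizontally along the world X axis within fixed bounds.
; On BeginPlay it adds the IMC_FaceMovement Enhanced Input mapping context to its player controller, and IA_Move feeds movement input along X.
; Every Tick it clamps the capsule's world location, limiting X to a set range and pinning Y and Z to constant values.
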(event Input|EnhancedActionEvents|EnhancedInputActionIA_Move
  (params (ActionValue :type Float%20%28double-precision%29) (ElapsedSeconds :type Float%20%28double-precision%29) (TriggeredSeconds :type Float%20%28double-precision%29) (InputAction :type Input%20Action%20Object%20Reference :default "/Game/Dynamic/Input/Actions/IA_Move.IA_Move"))
  (Pawn|Input|AddMovementInput "1.000000,0.000000,0.000000" ActionValue false))

(event EventBeginPlay
  (CallFunction|EnchancedMovementInput))

(event Collision|EventActorBeginOverlap
  (params (OtherActor :type Actor%20Object%20Reference)))

(event EventTick
  (params (DeltaSeconds :type Float%20%28single-precision%29))
  (bind _capsulecomponent (Variables|Default|GetCapsuleComponent))
  (bind _returnvalue (Transformation|GetWorldLocation _capsulecomponent))
  (bind _output_get (Variables|Default|SetfaceClamp (Math|Vector|MakeVector (Math|Float|Clamp(Float) (.x _returnvalue) -1678.0 1672.0) (Math|Float|Clamp(Float) (.y _returnvalue) 637.5 637.5) (Math|Float|Clamp(Float) (.z _returnvalue) -1057.5 -1057.5))))
  (Transformation|SetWorldLocation (Variables|Default|GetCapsuleComponent) _output_get false false))

(fn ConstructionScript)

(fn EnchancedMovementInput
  (bind _asplayer_controller (Utilities|Casting|CastToPlayerController (Pawn|GetController)))
  (Input|AddMappingContext (PlayerController|LocalPlayerSubsystems|GetEnhancedInputLocalPlayerSubsystem _asplayer_controller) "/Game/Dynamic/Input/IMC_FaceMovement.IMC_FaceMovement" 0 "(bIgnoreAllPressedKeysUntilRelease=True,bForceImmediately=False,bNotifyUserSettings=False)"))