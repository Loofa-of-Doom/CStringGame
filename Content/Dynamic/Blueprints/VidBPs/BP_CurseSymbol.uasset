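; BP_CurseSymbol is a curse-symbol pickup whose mesh is set from its picked symbol on BeginPlay.
; Each instance runs a looping timer that spawns another symbol at a start location.
; Tick clamps it to a fixed-depth play area and destroys it at the death zone.
; Hitting a "Face"-tagged actor destroys it, first advancing BP_MySeaString and moving or resetting the Text_Renderer arrow if it matches the selected symbol.
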(event Custom|Time%20To%20Spawn_Event
  (CallFunction|SpawnCurse))

(event EventBeginPlay
  (bind _symoblmesh (Variables|Default|GetSymoblMesh))
  (Utilities|Time|SetTimerbyEvent (delegate Custom|Time%20To%20Spawn_Event) 3.0 true)
  (switch Utilities|FlowControl|Switch|SwitchonCurseNames (Utilities|Enum|ByteToEnumCurseNames (Math|Conversions|ToByte(Integer) (Class|CurseSymbol|GetPickedSymbol self)))
    (:Defualt
      (Components|StaticMesh|SetStaticMesh _symoblmesh "/Game/Static/Props/SM_Bush.SM_Bush"))
    (:ExclamationPoint
      (Components|StaticMesh|SetStaticMesh _symoblmesh "/Game/Static/VidMesh/BlenderStuff/FullCheck.FullCheck"))
    (:Pound
      (Components|StaticMesh|SetStaticMesh _symoblmesh "/Game/Static/VidMesh/pound/PoundSymbol-1smol_fbx_Collection.PoundSymbol-1smol_fbx_Collection"))
    (:Ampersand
      (Components|StaticMesh|SetStaticMesh _symoblmesh "/Game/Static/VidMesh/ampersand/MidAmper.MidAmper"))
    (:Slash
      (Components|StaticMesh|SetStaticMesh _symoblmesh "/Game/Static/VidMesh/Slash/biggeron_s_sword.biggeron_s_sword"))
    (:MoneySign
      (Components|StaticMesh|SetStaticMesh _symoblmesh "/Game/Static/VidMesh/moneysign/CBFD_MoneyBag/MoneyBag.MoneyBag"))
    (:Questionmark
      (Components|StaticMesh|SetStaticMesh _symoblmesh "/Game/Static/VidMesh/question/Question_Mark/QuestionMark.QuestionMark"))))

(event Collision|EventActorBeginOverlap
  (params (OtherActor :type Actor%20Object%20Reference)))

(event EventTick
  (params (DeltaSeconds :type Float%20%28single-precision%29))
  (bind _capsule (Variables|Default|GetCapsule))
  (bind _returnvalue (Transformation|GetWorldLocation _capsule))
  (Transformation|SetWorldLocation (Variables|Default|GetCapsule) (Math|Vector|MakeVector (Math|Float|Clamp(Float) (.x _returnvalue) -1678.0 1672.0) (Math|Float|Clamp(Float) (.y _returnvalue) 637.5 637.5) (Math|Float|Clamp(Float) (.z _returnvalue) (Variables|Default|GetCurse%20Death%20Zone) 2.19e+03)) false false)
  (if (<= (.z (Transformation|GetActorLocation self)) (Variables|Default|GetCurse%20Death%20Zone))
    (Actor|DestroyActor)))

(event Collision|EventHit
  (params (MyComp :type Primitive%20Component%20Object%20Reference) (Other :type Actor%20Object%20Reference) (OtherComp :type Primitive%20Component%20Object%20Reference) (bSelfMoved :type Boolean) (HitLocation :type Vector :default "0, 0, 0") (HitNormal :type Vector :default "0, 0, 0") (NormalImpulse :type Vector :default "0, 0, 0") (Hit :type Hit%20Result%20Structure%20%28by%20ref%29))
  (if (Actor|ActorHasTag Other "Face")
    (bind _returnvalue (Actor|GetActorOfClass "/Game/Dynamic/Blueprints/VidBPs/BP_MySeaString.BP_MySeaString_C"))
    (if (== (Class|CurseSymbol|GetPickedSymbol self) (Class|SeaString|GetSelectedSymbol _returnvalue))
      (Class|SeaString|MoveSelectedSymbol _returnvalue)
      (bind _returnvalue_2 (Actor|GetActorOfClass "/Game/Dynamic/Blueprints/VidBPs/BP_MySeaString.BP_MySeaString_C"))
      (if (== (Class|SeaString|GetCurrentInd _returnvalue_2) 0)
        (bind _returnvalue_3 (Actor|GetActorOfClass "/Game/Dynamic/Blueprints/VidBPs/Text_Renderer.Text_Renderer_C"))
        (Default|ResetArrowLoc _returnvalue_3)
        (else
          (bind _returnvalue_4 (Actor|GetActorOfClass "/Game/Dynamic/Blueprints/VidBPs/Text_Renderer.Text_Renderer_C"))
          (Default|MoveArrow _returnvalue_4)))
      (Actor|DestroyActor)
      (else
        (Actor|DestroyActor)))))

(fn ConstructionScript)

(fn SpawnCurse
  (bind _returnvalue (Class|CurseSymbol|GetStartLocation))
  (Development|PrintString (Utilities|String|ToString(Vector) _returnvalue))
  (Game|SpawnActorfromClass "BP_CurseSymbol_C" (Math|Transform|MakeTransform _returnvalue) "Undefined" "MultiplyWithRoot" 0 0))