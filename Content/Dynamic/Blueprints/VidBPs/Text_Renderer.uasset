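; Text renderer actor that displays the word from BP_MySeaString at the BP_CharacterFace actor's location.
; On BeginPlay it attaches itself to BP_CharacterFace, then each Tick moves to that parent's location.
; Tick also looks up BP_MySeaString, splits and rejoins its FWord with empty separators, and writes it to TextRender.
; Helpers that offset an Arrow2 component exist, but their calls in the event graph never run.
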(event EventBeginPlay
  (bind _returnvalue (Actor|GetActorOfClass "/Game/Dynamic/Blueprints/VidBPs/BP_CharacterFace.BP_CharacterFace_C"))
  (Transformation|AttachActorToActor self _returnvalue "None" "KeepRelative" "KeepRelative" "KeepRelative" true))

(event EventTick
  (params (DeltaSeconds :type Float%20%28single-precision%29))
  (bind _returnvalue (Actor|GetActorOfClass "/Game/Dynamic/Blueprints/VidBPs/BP_MySeaString.BP_MySeaString_C"))
  (bind _returnvalue_2 (Class|SeaString|GetFWord _returnvalue))
  (Rendering|Components|TextRender|SetText (Variables|Default|GetTextRender) (Utilities|Text|ToText(String) (Utilities|String|JoinStringArray (Utilities|String|ParseIntoArray _returnvalue_2 " " false) " ")))
  (Transformation|SetActorLocation (Transformation|GetActorLocation (Actor|GetAttachParentActor self)) false false)
  (if true
    _))

(fn ConstructionScript)

(fn ResetArrowLoc
  (Transformation|AddWorldOffset (Variables|Default|Getarrow2) (Variables|Default|GetarrowStartLoc) false false))

(fn MoveArrow
  (Transformation|AddWorldOffset (Variables|Default|Getarrow2) (Variables|Default|GetmoveArrowDistance) false false))